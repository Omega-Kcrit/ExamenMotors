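; Door Blueprint that rises while the third-person character overlaps it, provided the game mode holds at least two coins.
; Overlap begin sets the Abriendose flag after the coin check, and any overlap end clears it.
; Tick calls Subir or Bajar from that flag, moving the static mesh vertically at constant, frame-rate-independent speed between the AlturaInicial and AlturaFinal height limits.
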(event `self.ReceiveActorBeginOverlap`
  (params (OtherActor :type "Actor Object Reference"))
  (cast `/Game/ThirdPersonBP/Blueprints/ThirdPersonCharacter` OtherActor)
  (bind _asthird_person_game_mode (cast `/Game/ThirdPersonBP/Blueprints/ThirdPersonGameMode` (`GameplayStatics.GetGameMode`)))
  (if (>= (`/Game/ThirdPersonBP/Blueprints/ThirdPersonGameMode.Coins` _asthird_person_game_mode) 2)
    (set `self.Abriendose` true)))

(event `self.ReceiveActorEndOverlap`
  (params (OtherActor :type "Actor Object Reference"))
  (set `self.Abriendose` false))

(event `self.ReceiveTick`
  (params (DeltaSeconds :type "Float (single-precision)"))
  (if (`self.Abriendose`)
    (`self.Subir` DeltaSeconds)
    (else
      (`self.Bajar` DeltaSeconds))))

(fn `Bajar`
  (params (`Delta TIem` :type "Float (double-precision)"))
  (bind (_returnvalue_x _returnvalue_y _returnvalue_z) (`KismetMathLibrary.BreakVector` (`SceneComponent.K2_GetComponentLocation` (`self.StaticMeshComponent`))))
  (bind (_returnvalue_x_2 _returnvalue_y_2 _returnvalue_z_2) (`KismetMathLibrary.BreakVector` (`SceneComponent.K2_GetComponentLocation` (`self.StaticMeshComponent`))))
  (if (not (<= _returnvalue_z (`self.Altura inicial`)))
    (`SceneComponent.K2_SetWorldLocation` (`self.StaticMeshComponent`) (`KismetMathLibrary.MakeVector` _returnvalue_x_2 _returnvalue_y_2 (- _returnvalue_z_2 (* `Delta TIem` 100.0))) false false)))

(fn `Subir`
  (params (DeltaTime :type "Float (double-precision)"))
  (bind (_returnvalue_x _returnvalue_y _returnvalue_z) (`KismetMathLibrary.BreakVector` (`SceneComponent.K2_GetComponentLocation` (`self.StaticMeshComponent`))))
  (if (not (<= (`self.Altura Final`) _returnvalue_z))
    (`SceneComponent.K2_SetWorldLocation` (`self.StaticMeshComponent`) (`KismetMathLibrary.MakeVector` _returnvalue_x _returnvalue_y (+ (* DeltaTime 100.0) _returnvalue_z)) false false)))

(fn `UserConstructionScript`)