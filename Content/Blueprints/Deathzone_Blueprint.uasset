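; Damage zone actor that drains the player's Life while occupied and requests a respawn from ThirdPersonGameMode at zero.
; Overlapping a living ThirdPersonCharacter sets a damage flag, which any end overlap clears; one already out of Life is destroyed and respawned.
; While flagged, Tick uses a one-second Delay to pace fixed damage to player pawn 0, printing Life.
; Death during Tick calls Respawn without destroying the character.
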(event `self.ReceiveActorEndOverlap`
  (params (OtherActor :type "Actor Object Reference"))
  (set `self.Damege` false))

(event `self.ReceiveActorBeginOverlap`
  (params (OtherActor :type "Actor Object Reference"))
  (bind _asthird_person_character (cast `/Game/ThirdPersonBP/Blueprints/ThirdPersonCharacter` OtherActor))
  (if (<= (`/Game/ThirdPersonBP/Blueprints/ThirdPersonCharacter.Life` _asthird_person_character) 0.0)
    (`self.K2_DestroyActor` _asthird_person_character)
    (bind _asthird_person_game_mode (cast `/Game/ThirdPersonBP/Blueprints/ThirdPersonGameMode` (`GameplayStatics.GetGameMode`)))
    (`/Game/ThirdPersonBP/Blueprints/ThirdPersonGameMode.Respawn` _asthird_person_game_mode)
    (else
      (set `self.Damege` true))))

(event `self.ReceiveTick`
  (params (DeltaSeconds :type "Float (single-precision)"))
  (if (`self.Damege`)
    (bind _asthird_person_character (cast `/Game/ThirdPersonBP/Blueprints/ThirdPersonCharacter` (`GameplayStatics.GetPlayerPawn` 0)))
    (`KismetSystemLibrary.Delay` 1.0)
    (bind _output_get (set `/Game/ThirdPersonBP/Blueprints/ThirdPersonCharacter.Life` (- (`/Game/ThirdPersonBP/Blueprints/ThirdPersonCharacter.Life` _asthird_person_character) 25.0) _asthird_person_character))
    (`KismetSystemLibrary.PrintString` (`KismetStringLibrary.Conv_DoubleToString` _output_get))
    (if (<= (`/Game/ThirdPersonBP/Blueprints/ThirdPersonCharacter.Life` _asthird_person_character) 0.0)
      (bind _asthird_person_game_mode (cast `/Game/ThirdPersonBP/Blueprints/ThirdPersonGameMode` (`GameplayStatics.GetGameMode`)))
      (`/Game/ThirdPersonBP/Blueprints/ThirdPersonGameMode.Respawn` _asthird_person_game_mode))))

(fn `UserConstructionScript`)