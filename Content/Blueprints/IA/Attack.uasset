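; Behavior tree task that makes an AI attack the player character.
; After a one-second delay it subtracts a fixed amount from the player's Life and prints the new value.
; When Life reaches zero or below it calls Respawn on the ThirdPersonGameMode.
; It then finishes with success, but a failed cast leaves the task unfinished.
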(event `self.ReceiveExecuteAI`
  (params (OwnerController :type "AIController Object Reference") (ControlledPawn :type "Pawn Object Reference"))
  (bind _asthird_person_character (cast `/Game/ThirdPersonBP/Blueprints/ThirdPersonCharacter` (`GameplayStatics.GetPlayerPawn` 0)))
  (`KismetSystemLibrary.Delay` 1.0)
  (bind _output_get (set `/Game/ThirdPersonBP/Blueprints/ThirdPersonCharacter.Life` (- (`/Game/ThirdPersonBP/Blueprints/ThirdPersonCharacter.Life` _asthird_person_character) 25.0) _asthird_person_character))
  (`KismetSystemLibrary.PrintString` (`KismetStringLibrary.Conv_DoubleToString` _output_get))
  (if (<= (`/Game/ThirdPersonBP/Blueprints/ThirdPersonCharacter.Life` _asthird_person_character) 0.0)
    (bind _asthird_person_game_mode (cast `/Game/ThirdPersonBP/Blueprints/ThirdPersonGameMode` (`GameplayStatics.GetGameMode`)))
    (`/Game/ThirdPersonBP/Blueprints/ThirdPersonGameMode.Respawn` _asthird_person_game_mode)
    (`self.FinishExecute` true)
    (else
      (`self.FinishExecute` true))))